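; BP_Enemy is a shooter enemy that periodically fires at the player and can be destroyed by damage.
; A looping timer started on BeginPlay spawns BP_Enemy_Projectile at the enemy's location, rotated toward the player pawn's current position.
; AnyDamage subtracts from HP and prints it.
; At zero or below, it disables collision, spawns BP_Enemy_Death, plays a pitched-up death sound and destroys itself.
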(event `self.ReceiveBeginPlay`
  (`KismetSystemLibrary.K2_SetTimerDelegate` (delegate `SpawnProjectile`) 1.0 true))

(event `SpawnProjectile`
  (`|SpawnActorFromClass` "/Game/TateShoot/BP_Enemy_Projectile.BP_Enemy_Projectile_C" (`KismetMathLibrary.MakeTransform` (`self.K2_GetActorLocation`) (`KismetMathLibrary.FindLookAtRotation` (`self.K2_GetActorLocation`) (`self.K2_GetActorLocation` (`GameplayStatics.GetPlayerPawn` 0)))) "Undefined" "OverrideRootScale" null null))

(event `self.ReceiveAnyDamage`
  (params (Damage :type "Float (single-precision)") (DamageType :type "DamageType Object Reference") (InstigatedBy :type "Controller Object Reference") (DamageCauser :type "Actor Object Reference"))
  (bind _output_get (set `self.HP` (- (`self.HP`) Damage)))
  (`KismetSystemLibrary.PrintString` (`KismetStringLibrary.Conv_DoubleToString` _output_get))
  (if (not (> _output_get 0.0))
    (`self.SetActorEnableCollision` false)
    (`|SpawnActorFromClass` "/Game/TateShoot/FX/BP_Enemy_Death.BP_Enemy_Death_C" (`self.GetTransform`) "Undefined" "OverrideRootScale" null null)
    (`GameplayStatics.SpawnSound2D` "/Game/TateShoot/Sound/SE_Death.SE_Death" 1.0 1.5 0.0 null)
    (`self.K2_DestroyActor`)))

(fn `UserConstructionScript`)