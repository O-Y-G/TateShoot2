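; BP_Player is the player in a shooter, moving along fixed world X and Y axes and firing projectiles.
; Holding Shoot fires immediately, then repeats on a looping timer until release or death.
; Damage decrements and prints Life, spawns a death actor, hides the player and disables input and collision.
; After a delay it respawns at its start position with brief invincibility; Life is never checked for game over.
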(event `self.ReceiveBeginPlay`
  (set `self.StartPos` (`self.K2_GetActorLocation`)))

(event `InputAxis|MoveForward`
  (params (AxisValue :type "Float (single-precision)"))
  (`self.AddMovementInput` (0.0 1.0 0.0) AxisValue))

(event `InputAxis|MoveRight`
  (params (AxisValue :type "Float (single-precision)"))
  (`self.AddMovementInput` (1.0 0.0 0.0) AxisValue))

(event `InputAction|Shoot`
  (params (Key :type "Key Structure"))
  (:`Pressed`
    (if (not (`self.bDeath`))
      (bind _returnvalue (`KismetSystemLibrary.K2_SetTimerDelegate` (delegate `ShootLoop`) 0.1 true))
      (set `self.ShootTimer` _returnvalue)
      (`self.ShootLoop`)))
  (:`Released`
    (`KismetSystemLibrary.K2_ClearAndInvalidateTimerHandle` (`self.ShootTimer`))))

(event `ShootLoop`
  (`|SpawnActorFromClass` "/Game/TateShoot/BP_Player_Projectile.BP_Player_Projectile_C" (`self.GetTransform`) "Undefined" "OverrideRootScale" null null)
  (`GameplayStatics.SpawnSound2D` "/Game/TateShoot/Sound/SE_Shoot.SE_Shoot" 1.0 1.0 0.0 null))

(event `self.ReceiveAnyDamage`
  (params (Damage :type "Float (single-precision)") (DamageType :type "DamageType Object Reference") (InstigatedBy :type "Controller Object Reference") (DamageCauser :type "Actor Object Reference"))
  (if (not (`self.bInvincible`))
    (bind _result (`/Engine/EditorBlueprintResources/StandardMacros.DecrementInt` (`self.Life`))
      (:`  `
        (`KismetSystemLibrary.PrintString` (`KismetStringLibrary.Conv_IntToString` _result))
        (set `self.bInvincible` true)
        (set `self.bDeath` true)
        (`self.DisableInput` null)
        (`self.SetActorEnableCollision` false)
        (`|SpawnActorFromClass` "/Game/TateShoot/FX/BP_Player_Death.BP_Player_Death_C" (`self.GetTransform`) "Undefined" "OverrideRootScale" null null)
        (`GameplayStatics.SpawnSound2D` "/Game/TateShoot/Sound/SE_Death.SE_Death" 1.0 1.0 0.0 null)
        (`SceneComponent.SetHiddenInGame` (`self.Scene`) true true)
        (`KismetSystemLibrary.K2_ClearAndInvalidateTimerHandle` (`self.ShootTimer`))
        (`KismetSystemLibrary.Delay` 2.0)
        (`self.K2_SetActorLocation` (`self.StartPos`))
        (`SceneComponent.SetHiddenInGame` (`self.Scene`) false true)
        (set `self.bDeath` false)
        (`self.SetActorEnableCollision` true)
        (`self.EnableInput` null)
        (`KismetSystemLibrary.Delay` 2.0)
        (set `self.bInvincible` false)))))

(fn `UserConstructionScript`)